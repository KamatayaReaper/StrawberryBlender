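; Player controller for Strawberry Blender that sets up input and drives cursor-based aiming of the player pawn.
; On BeginPlay it adds the IMC_StrawberryBlender Enhanced Input mapping context, switches to game-only input and shows the mouse cursor.
; Every tick it traces under the cursor on the Visibility channel and passes the hit location to the pawn through SetRotationMessage, without checking whether the trace hit.
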(event `self.ReceiveBeginPlay`
  (bind _returnvalue (subsystem `EnhancedInputLocalPlayerSubsystem`))
  (`|ExecutionSequence`
    (:`then_0`
      (`/Engine/EditorBlueprintResources/StandardMacros.IsValid` _returnvalue
        (:`Is Valid`
          (`EnhancedInputSubsystemInterface.AddMappingContext` _returnvalue "/Game/StrawberryBlender/Inputs/IMC_StrawberryBlender.IMC_StrawberryBlender" 0 (struct)))))
    (:`then_1`
      (`WidgetBlueprintLibrary.SetInputMode_GameOnly` self)
      (set `self.bShowMouseCursor` true))))

(event `self.ReceiveTick`
  (params (DeltaSeconds :type "Float (single-precision)"))
  (message `/Game/StrawberryBlender/Blueprints/BPI_TopdownPlayer.SetRotation` (`GameplayStatics.GetPlayerPawn` 0) (`.Location` (`GameplayStatics.BreakHitResult` (`self.GetHitResultUnderCursorByChannel` "TraceTypeQuery1")))))

(fn `UserConstructionScript`)