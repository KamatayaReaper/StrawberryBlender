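; An animation notify state that opens the player's melee weapon active window during an animation.
; On begin it casts the mesh owner to the player character parent and calls WeaponActive on the melee weapon in its PlayerWeapon child actor.
; On end it calls WeaponDeactive on that weapon.
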(fn `Received_NotifyBegin`
  (params (MeshComp :type "SkeletalMeshComponent Object Reference") (Animation :type "AnimSequenceBase Object Reference") (TotalDuration :type "Float (single-precision)") (EventReference :type "AnimNotifyEventReference Structure (by ref)"))
  (returns (ReturnValue :type Boolean))
  (bind _asbp_player_character_parent (cast `/Game/StrawberryBlender/Blueprints/BP_PlayerCharacterParent` (`ActorComponent.GetOwner` MeshComp)))
  (bind _asbp_melee_weapon_parent (cast `/Game/StrawberryBlender/Blueprints/Weapons/BP_MeleeWeaponParent` (`ChildActorComponent.ChildActor` (`/Game/StrawberryBlender/Blueprints/BP_PlayerCharacterParent.PlayerWeapon` _asbp_player_character_parent))))
  (`/Game/StrawberryBlender/Blueprints/Weapons/BP_MeleeWeaponParent.WeaponActive` _asbp_melee_weapon_parent)
  (return false))

(fn `Received_NotifyEnd`
  (params (MeshComp :type "SkeletalMeshComponent Object Reference") (Animation :type "AnimSequenceBase Object Reference") (EventReference :type "AnimNotifyEventReference Structure (by ref)"))
  (returns (ReturnValue :type Boolean))
  (bind _asbp_player_character_parent (cast `/Game/StrawberryBlender/Blueprints/BP_PlayerCharacterParent` (`ActorComponent.GetOwner` MeshComp)))
  (bind _asbp_melee_weapon_parent (cast `/Game/StrawberryBlender/Blueprints/Weapons/BP_MeleeWeaponParent` (`ChildActorComponent.ChildActor` (`/Game/StrawberryBlender/Blueprints/BP_PlayerCharacterParent.PlayerWeapon` _asbp_player_character_parent))))
  (`/Game/StrawberryBlender/Blueprints/Weapons/BP_MeleeWeaponParent.WeaponDeactive` _asbp_melee_weapon_parent)
  (return false))