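; Base melee weapon Blueprint that damages enemies touched by its hit range while the weapon is active.
; WeaponActive and WeaponDeactive events toggle a flag that gates overlaps on the MeleeHitRange component.
; An overlapping actor other than the owner that implements BPI_Enemy receives WeaponDamage.
; A DoOnce reset after a short delay limits hits to one per cooldown, shared across all targets.
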(event `self.MeleeHitRange.OnComponentBeginOverlap`
  (params (OverlappedComponent :type "PrimitiveComponent Object Reference") (OtherActor :type "Actor Object Reference") (OtherComp :type "PrimitiveComponent Object Reference") (OtherBodyIndex :type Integer) (bFromSweep :type Boolean) (SweepResult :type "HitResult Structure (by ref)"))
  (if (and (!= OtherActor (`self.GetOwner`)) (`KismetSystemLibrary.DoesImplementInterface` OtherActor "/Game/StrawberryBlender/Blueprints/BPI_Enemy.BPI_Enemy_C") (`self.WeaponActive?`))
    (`/Engine/EditorBlueprintResources/StandardMacros.DoOnce` false :!label _label
      (:`Completed`
        (`GameplayStatics.ApplyDamage` OtherActor (`self.WeaponDamage`))
        (`KismetSystemLibrary.Delay` 0.5)
        (goto _label :!via `Reset`)))))

(event `WeaponActive`
  (set `self.WeaponActive?` true))

(event `WeaponDeactive`
  (set `self.WeaponActive?` false))

(fn `UserConstructionScript`)